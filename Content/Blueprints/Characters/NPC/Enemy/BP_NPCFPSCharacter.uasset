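; BP_NPCFPSCharacter is an enemy NPC character that equips a weapon and seeds its AI Blackboard when play begins.
; It attaches the weapon at the assault rifle grip point, then writes itself to the SelfActor key.
; The next point from its Patrol component goes into the PatrolPoint key, with a red error printed if no patrol points exist.
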(event EventBeginPlay
  (Class|FPSCharacter|SetWeapon "/Game/Blueprints/Weapons/Weapon_BP.Weapon_BP_C" "AssaultRifleGripPoint")
  (CallFunction|InitializePatrolKeys)
  (CallFunction|InitializeSelfKey))

(event Collision|EventActorBeginOverlap
  (params (OtherActor :type Actor%20Object%20Reference)))

(event EventTick
  (params (DeltaSeconds :type Float%20%28single-precision%29)))

(fn ConstructionScript)

(fn InitializePatrolKeys
  (bind _patrol (Variables|Default|GetPatrol))
  (bind _returnvalue (Class|PatrolComponent|GetPatrolPoints _patrol))
  (if (> (Utilities|Array|Length _returnvalue) 0)
    (AI|Components|Blackboard|SetValueasObject (AI|GetBlackboard (AI|GetAIController self)) (Utilities|Name|MakeLiteralName "PatrolPoint") (Utilities|Array|Get(acopy) _returnvalue (Class|PatrolComponent|GetNextPatrolPoint _patrol)))
    (else
      (Development|PrintString "ERROR: 0 patrol points" true true "(R=1.000000,G=0.000000,B=0.000000,A=1.000000)"))))

(fn InitializeSelfKey
  (bind _self self)
  (AI|Components|Blackboard|SetValueasObject (AI|GetBlackboard (AI|GetAIController _self)) (Utilities|Name|MakeLiteralName "SelfActor") _self))